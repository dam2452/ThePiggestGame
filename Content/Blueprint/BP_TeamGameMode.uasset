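; Team-based game mode that assigns joining players to teams round-robin, respawns them at their team's spawn points and tracks team score.
; On BeginPlay it creates team info objects in the game state; the authority fills them with PlayerStarts tagged "Team{ID}".
; Login and the KillPlayer timer both call RespawnPlayer, which picks a random team start and heals the character to full.
; EndGame is an empty stub.
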(event `self.K2_PostLogin`
  (params (NewPlayer :type "PlayerController Object Reference"))
  (`self.HandlePostLogin` NewPlayer)
  ;[1 1 1] Post Login
  (bind _asbp_player_controller (cast `/Game/Blueprint/BP_PlayerController` NewPlayer))
  (`self.AssignPlayerToTeam` _asbp_player_controller)
  (`self.RespawnPlayer` _asbp_player_controller))

(event `self.K2_OnLogout`
  (params (ExitingController :type "Controller Object Reference"))
  (`self.HandleLogout` ExitingController))

(event `self.ReceiveBeginPlay`
  (`self.Initialize Teams`)
  (`/Engine/EditorBlueprintResources/ActorMacros.Switch Has Authority`
    (:`Authority`
      (bind _asbp_team_game_state (cast `/Game/Blueprint/BP_TeamGameState` (`GameplayStatics.GetGameState`)))
      (set `self.As BP Team Game State` _asbp_team_game_state)
      (`self.UpdateTeamSpawnPoints`))))

(event `KillPlayer`
  (params (PlayerController :type "Controller Object Reference"))
  (`KismetSystemLibrary.K2_SetTimerDelegate` (delegate `Respawn`) (`self.RespawnTime`)))

(event `Respawn`
  (`self.RespawnPlayer` (stale `KillPlayer` PlayerController)))

(fn `AddScoreToTeam`
  (params (TeamId :type Integer) (Score :type "Float (double-precision)"))
  (bind _asbp_team_game_state (cast `/Game/Blueprint/BP_TeamGameState` (`GameplayStatics.GetGameState`)))
  (for _array_element (`/Game/Blueprint/BP_TeamGameState.Teams Info` _asbp_team_game_state)
    (if (== (`/Game/Blueprint/BP_TeamInfo.TeamId` _array_element) (`local.TeamId`))
      (`/Game/Blueprint/BP_TeamInfo.AddScore` _array_element (`local.Score`)))))

(fn `AssignPlayerToTeam`
  (params (PlayerController :type "Controller Object Reference"))
  (`/Engine/EditorBlueprintResources/StandardMacros.IsValid` PlayerController
    (:`Is Valid`
      (bind _asbp_team_player_state (cast `/Game/Blueprint/BP_TeamPlayerState` (`Controller.PlayerState` PlayerController)))
      (`/Game/Blueprint/BP_TeamPlayerState.SetTeamId` _asbp_team_player_state (+ (mod (`self.AssignedPlayerCount `) (`self.MaxTeams`)) 1))
      (`/Engine/EditorBlueprintResources/StandardMacros.IncrementInt` (`self.AssignedPlayerCount `)))))

(fn `EndGame`)

(fn `Initialize Teams`
  (for _index (range 1 (+ (`self.MaxTeams`) 1))
    (bind _returnvalue (`|GenericCreateObject` "/Game/Blueprint/BP_TeamInfo.BP_TeamInfo_C"))
    (`/Game/Blueprint/BP_TeamInfo.SetTeamId` _returnvalue _index)
    (bind _asbp_team_game_state (cast `/Game/Blueprint/BP_TeamGameState` (`GameplayStatics.GetGameState`)))
    (`KismetArrayLibrary.Array_Add` (`/Game/Blueprint/BP_TeamGameState.Teams Info` _asbp_team_game_state) _returnvalue)))

(fn `RespawnPlayer`
  (params (PlayerController :type "Controller Object Reference"))
  (locals (PlayerStarts :type "Array of Actor Object Reference") (TeamTag :type String) (FilteredStarts :type "Array of Actor Object Reference") (TeamIdLocal :type Integer :default 0))
  (bind _playercontroller (`local.PlayerController`))
  (bind _asbp_team_player_state (cast `/Game/Blueprint/BP_TeamPlayerState` (`Controller.PlayerState` PlayerController)))
  (set `local.TeamIdLocal` (`/Game/Blueprint/BP_TeamPlayerState.TeamId ` _asbp_team_player_state))
  (`/Engine/EditorBlueprintResources/StandardMacros.IsValid` PlayerController
    (:`Is Valid`
      (`/Engine/EditorBlueprintResources/StandardMacros.IsValid` (`self.As BP Team Game State`)
        (:`Is Valid`
          (for _array_element (`/Game/Blueprint/BP_TeamGameState.Teams Info` (`self.As BP Team Game State`))
            (if (== (`/Game/Blueprint/BP_TeamInfo.TeamId` _array_element) (`local.TeamIdLocal`))
              (bind _respawnpoints (`/Game/Blueprint/BP_TeamInfo.RespawnPoints` _array_element))
              (`self.RestartPlayerAtPlayerStart` _playercontroller (`|GetArrayItem` _respawnpoints (`KismetMathLibrary.RandomIntegerInRange` 0 (- (`KismetArrayLibrary.Array_Length` _respawnpoints) 1))))
              (bind _asbp_top_down_char (cast `/Game/Character/BP_TopDownChar` (`Controller.K2_GetPawn` _playercontroller)))
              (bind _bpc_healthcomponent (`/Game/Character/BP_TopDownChar.BPC_HealthComponent` _asbp_top_down_char))
              ;[1 1 1] TODO
              (`/Game/Blueprint/BPC_HealthComponent.MC_Heal` _bpc_healthcomponent (`/Game/Blueprint/BPC_HealthComponent.MaxHealth` _bpc_healthcomponent)))))))))

(fn `SetPlayerVisible`
  (params (Visible :type Boolean) (Controller :type "Controller Object Reference"))
  ;[1 1 1] TODO
  (bind _asbp_top_down_char (cast `/Game/Character/BP_TopDownChar` (`Controller.K2_GetPawn` Controller)))
  (if Visible
    (bind _rootcomponent (`Actor.RootComponent` _asbp_top_down_char))
    (`SceneComponent.SetVisibility` _rootcomponent true true)
    (else
      (`SceneComponent.SetVisibility` _rootcomponent false true))))

(fn `UpdateTeamSpawnPoints`
  (locals (SpawnPoints :type "Array of PlayerStart Object Reference"))
  (bind _outactors (`GameplayStatics.GetAllActorsOfClass` "/Script/Engine.PlayerStart"))
  (bind _output_get (set `local.SpawnPoints` _outactors))
  (for _array_element (`/Game/Blueprint/BP_TeamGameState.Teams Info` (`self.As BP Team Game State`))
    (for _array_element_2 _output_get
      (if (`self.ActorHasTag` _array_element_2 (`KismetStringLibrary.Conv_StringToName` (`KismetTextLibrary.Conv_TextToString` (`|FormatText` "Team{ID}" (`/Game/Blueprint/BP_TeamInfo.TeamId` _array_element)))))
        (`/Game/Blueprint/BP_TeamInfo.AddRespawnPoint` _array_element _array_element_2)))))

(fn `UserConstructionScript`)