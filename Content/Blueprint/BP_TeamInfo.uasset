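; BP_TeamInfo holds the data for one team: its ID, score and respawn points.
; Simple functions set the ID, add points to the score and register respawn points.
; GetRandomRespawnPoint picks a random entry from the registered points and returns an empty result when none exist.
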(fn `AddRespawnPoint`
  (params (RespawnPoint :type "Actor Object Reference (by ref)"))
  (`KismetArrayLibrary.Array_Add` (`self.RespawnPoints`) RespawnPoint))

(fn `AddScore`
  (params (Points :type "Float (double-precision)"))
  (set `self.Score` (+ Points (`self.Score`))))

(fn `GetRandomRespawnPoint`
  (returns (RandomRespawnPoint :type "Actor Object Reference"))
  (locals (RespawnPointsLengthLocal :type Integer :default 0))
  (bind _output_get (set `local.RespawnPointsLengthLocal` (`KismetArrayLibrary.Array_Length` (`self.RespawnPoints`))))
  (if (> _output_get 0)
    (return (`|GetArrayItem` (`self.RespawnPoints`) (`KismetMathLibrary.RandomIntegerInRange` 0 (- (`local.RespawnPointsLengthLocal`) 1))))
    (else
      (return null))))

(fn `SetTeamId`
  (params (NewTeamId :type Integer))
  (set `self.TeamId` NewTeamId))