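; Player controller that sets up the local player's HUD and provides a score printout on demand.
; On BeginPlay, it creates WBP_HeadsUpDisplay for local controllers only, stores it and adds it to the viewport.
; Pressing Tab calls SR_DrawScores, which loops over the GameState PlayerArray, casts each entry to BP_PlayerState and prints its player ID and score as debug text.
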(event `self.ReceiveBeginPlay`
  (if (`self.IsLocalPlayerController`)
    (bind _returnvalue (`|CreateWidget` "/Game/Blueprint/WBP_HeadsUpDisplay.WBP_HeadsUpDisplay_C"))
    (bind _output_get (set `self.HeadsUpDisplay` _returnvalue))
    (`UserWidget.AddToViewport` _output_get 0)))

(event `SR_DrawScores`
  (for _array_element (`GameStateBase.PlayerArray` (`GameplayStatics.GetGameState`))
    (bind _asbp_player_state (cast `/Game/Blueprint/BP_PlayerState` _array_element))
    (`KismetSystemLibrary.PrintString` (`KismetTextLibrary.Conv_TextToString` (`|FormatText` "Player ID: {id}       Score: {score}" (`PlayerState.PlayerId` _asbp_player_state) (`/Game/Blueprint/BP_PlayerState.Player Score` _asbp_player_state))) true true (struct :`R` 1.0 :`B` 0.07889 :`A` 1.0))))

(event `Key|Tab`
  (params (Key :type "Key Structure"))
  (:`Pressed`
    (`self.SR_DrawScores`)))

(fn `UserConstructionScript`)