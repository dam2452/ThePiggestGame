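; BP_Utilities is a set of grid helper functions for a Paper2D tile map game, working on the world XY plane.
; Tile size lookup and world-to-tile conversion read tile dimensions from the first PaperTileMapActor found through GetAllActorsOfClass.
; Conversion divides and rounds to the nearest index, ignoring the map actor's transform.
; SnapToGrid independently rounds X and Y to a supplied uniform tile size, preserving Z.
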(fn `Convert World Position to Tile`
  (params (WorldPosition :type "Vector Structure"))
  (returns (TilePosition :type "IntPoint Structure"))
  (locals (`TileX ` :type Integer :default 20) (TileY :type Integer) (`Map Width` :type Integer :default 0) (`Map Height` :type Integer :default 0) (`World Position` :type "Vector Structure"))
  (bind _world_position_x (`KismetMathLibrary.BreakVector` (`local.World Position`)))
  (bind (_world_position_x_2 _world_position_y) (`KismetMathLibrary.BreakVector` (`local.World Position`)))
  (set `local.World Position` WorldPosition)
  (bind _outactors (`GameplayStatics.GetAllActorsOfClass` null "/Script/Paper2D.PaperTileMapActor"))
  (bind _tilemap (`PaperTileMapComponent.TileMap` (`PaperTileMapActor.RenderComponent` (`|GetArrayItem` _outactors))))
  (set `local.TileY` (`KismetMathLibrary.Round` (/ _world_position_y (`PaperTileMap.TileHeight` _tilemap))))
  (set `local.TileX ` (`KismetMathLibrary.Round` (/ _world_position_x (`PaperTileMap.TileWidth` _tilemap))))
  (return (make `IntPoint` (`local.TileX `) (`local.TileY`))))

(fn `Get Tile Size`
  (returns (`Tile Size` :type "IntPoint Structure"))
  (bind _outactors (`GameplayStatics.GetAllActorsOfClass` null "/Script/Paper2D.PaperTileMapActor"))
  (bind _tilemap (`PaperTileMapComponent.TileMap` (`PaperTileMapActor.RenderComponent` (`|GetArrayItem` _outactors))))
  (return (make `IntPoint` (`PaperTileMap.TileWidth` _tilemap) (`PaperTileMap.TileHeight` _tilemap))))

(fn `SnapToGrid`
  (params (Location :type "Vector Structure") (`Tile Size` :type Integer :default 32))
  (returns (`Snapped Location` :type "Vector Structure"))
  (return (`KismetMathLibrary.MakeVector` (* (`KismetMathLibrary.Round` (/ (.x Location) `Tile Size`)) `Tile Size`) (* (`KismetMathLibrary.Round` (/ (.y Location) `Tile Size`)) `Tile Size`) (.z Location))))