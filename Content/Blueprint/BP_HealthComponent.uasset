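; BP_HealthComponent is a health component that tracks Health, starting at MaxHealth, and reports to the team game mode when damaged.
; TakeDamage subtracts clamped damage on the authority, skipping only when the owner is dead and damage is non-positive.
; It then calls KillPlayer on BP_TeamGameMode with team 0, without checking remaining health, if the top-down character and team player state casts succeed.
; Heal is an empty stub.
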(event `self.ReceiveBeginPlay`
  (set `self.Health` (`self.MaxHealth`)))

(fn `Heal`)

(fn `IsAlive`
  (returns (IsAlive :type Boolean))
  (return (> (`self.Health`) 0.0)))

(fn `TakeDamage`
  (params (Damage :type "Float (double-precision)"))
  (if (not (and (not (`self.IsAlive`)) (<= Damage 0.0)))
    (`/Engine/EditorBlueprintResources/ActorComponentMacros.Switch Has Authority`
      (:`Authority`
        (set `self.Health` (`KismetMathLibrary.FClamp` (- (`self.Health`) (`local.Damage`)) 0.0 (`self.MaxHealth`)))
        (bind _asbp_team_game_mode (cast `/Game/Blueprint/BP_TeamGameMode` (`GameplayStatics.GetGameMode`)))
        (bind _asbp_top_down_char (cast `/Game/Character/BP_TopDownChar` (`self.GetOwner`)))
        (cast `/Game/Blueprint/BP_TeamPlayerState` (`Controller.PlayerState` (`Pawn.GetController` _asbp_top_down_char)))
        (`/Game/Blueprint/BP_TeamGameMode.KillPlayer` _asbp_team_game_mode null 0)))))