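; Game mode that keeps a list of player controllers and builds a multiplayer scoreboard from each player state's name and score.
; Login and logout handlers update the list and refresh the scoreboard, but their EventGraph calls are unconnected.
; UpdateScoreboardGM attempts a highest-first selection sort, though its running maximum is only assigned to itself.
; The resulting array is pushed to every BP_PlayerController.
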(fn `HandleLogout`
  (params (Controller :type "Controller Object Reference"))
  (bind _asplayer_controller (cast `PlayerController` Controller))
  (`KismetArrayLibrary.Array_RemoveItem` (`self.AllPCs`) _asplayer_controller)
  (`self.UpdateScoreboardGM`))

(fn `HandlePostLogin`
  (params (Controller :type "PlayerController Object Reference (by ref)"))
  (`KismetArrayLibrary.Array_Add` (`self.AllPCs`) Controller)
  (`self.UpdateScoreboardGM`))

(fn `UpdateScoreboardGM`
  (locals (PlayerEntryCopyLocal :type "Array of /Game/Blueprint/F_ScoreboardEntryStruct Structure") (LoopBiggestScore :type "Float (double-precision)") (LoopBiggestScoreIndex :type Integer))
  (bind _loopbiggestscore (`local.LoopBiggestScore`))
  (`KismetArrayLibrary.Array_Clear` (`self.PlayerEntry`))
  (for _array_element (`self.AllPCs`)
    (bind _asbp_player_state (cast `/Game/Blueprint/BP_PlayerState` (`Controller.PlayerState` _array_element)))
    (`KismetArrayLibrary.Array_Add` (`self.PlayerEntry`) (make `/Game/Blueprint/F_ScoreboardEntryStruct` (`PlayerState.GetPlayerName` _asbp_player_state) (`/Game/Blueprint/BP_PlayerState.Player Score` _asbp_player_state))))
  ;[1 1 1] Sorting (ctrl c ctrl v)
  (`KismetArrayLibrary.Array_Clear` (`self.PlayerEntrySorted`))
  (bind _output_get (set `local.PlayerEntryCopyLocal` (`self.PlayerEntry`)))
  (if (> (`KismetArrayLibrary.Array_Length` _output_get) 0) :!label _label
    (for (_array_element_2 _array_index) (`local.PlayerEntryCopyLocal`)
      (if (or (> (`.Score_6_80C03F2D494B868A1BA3D3A4B83A48A8` (break `/Game/Blueprint/F_ScoreboardEntryStruct` _array_element_2)) _loopbiggestscore) (== _array_index 0))
        (set `local.LoopBiggestScore` _loopbiggestscore)
        (set `local.LoopBiggestScoreIndex` _array_index)))
    (`KismetArrayLibrary.Array_Add` (`self.PlayerEntrySorted`) (`|GetArrayItem` (`local.PlayerEntryCopyLocal`) (`local.LoopBiggestScoreIndex`)))
    (`KismetArrayLibrary.Array_Remove` (`local.PlayerEntryCopyLocal`) (`local.LoopBiggestScoreIndex`))
    (goto _label)
    (else
      (for _array_element_3 (`self.AllPCs`)
        (bind _asbp_player_controller (cast `/Game/Blueprint/BP_PlayerController` _array_element_3))
        (`/Game/Blueprint/BP_PlayerController.UpdateScoreboard` _asbp_player_controller (`self.PlayerEntrySorted`))))))

(fn `UserConstructionScript`)