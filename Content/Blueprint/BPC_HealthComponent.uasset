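; Health component for a top-down team game character that tracks health, applies damage and healing, and reports death.
; TakeDamage ignores dead owners and non-positive amounts, clamps Health, and at zero has BP_TeamGameMode kill the instigator's controller, then updates the HUD.
; Heal, also exposed through the MC_Heal event, runs if alive or the amount is positive, so it can revive, then calls MCCallUpdateHUD on BP_TopDownChar.
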(event `self.ReceiveBeginPlay`
  (set `self.Health` (`self.MaxHealth`)))

(event `MC_Heal`
  (params (Heal :type "Float (double-precision)"))
  (`self.Heal` Heal))

(fn `Heal`
  (params (Heal :type "Float (double-precision)"))
  (if (or (`self.IsAlive`) (not (<= Heal 0.0)))
    (set `self.Health` (`KismetMathLibrary.FClamp` (+ (`self.Health`) Heal) 0.0 (`self.MaxHealth`)))
    (bind _asbp_top_down_char (cast `/Game/Character/BP_TopDownChar` (`self.GetOwner`)))
    (`/Game/Character/BP_TopDownChar.MC_CallUpdateHUD` _asbp_top_down_char)))

(fn `IsAlive`
  (returns (IsAlive :type Boolean))
  (return (> (`self.Health`) 0.0)))

(fn `TakeDamage`
  (params (Damage :type "Float (double-precision)"))
  (if (not (or (not (`self.IsAlive`)) (<= Damage 0.0)))
    (bind _output_get (set `self.Health` (`KismetMathLibrary.FClamp` (- (`self.Health`) (`local.Damage`)) 0.0 (`self.MaxHealth`))))
    (if (<= _output_get 0.0)
      (bind _asbp_team_game_mode (cast `/Game/Blueprint/BP_TeamGameMode` (`GameplayStatics.GetGameMode`)))
      (`/Game/Blueprint/BP_TeamGameMode.KillPlayer` _asbp_team_game_mode (`Pawn.GetController` (`Actor.Instigator` (`self.GetOwner`))))
      (bind _asbp_top_down_char (cast `/Game/Character/BP_TopDownChar` (`self.GetOwner`)))
      (`/Game/Character/BP_TopDownChar.MC_CallUpdateHUD` _asbp_top_down_char))))