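; BP_Pickup is a sprite-based collectible that raises the score when a BP_TopDownChar touches it.
; The construction script sizes its box collision slightly larger than the sprite's bounds.
; On overlap, the authority destroys the pickup, then increments the score widget on player controller 0's BP_HUD, regardless of which character collected it.
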(event `self.PickupCollision.OnComponentBeginOverlap`
  (params (OverlappedComponent :type "PrimitiveComponent Object Reference") (OtherActor :type "Actor Object Reference") (OtherComp :type "PrimitiveComponent Object Reference") (OtherBodyIndex :type Integer) (bFromSweep :type Boolean) (SweepResult :type "HitResult Structure (by ref)"))
  (`/Engine/EditorBlueprintResources/ActorMacros.Switch Has Authority`
    (:`Authority`
      (bind _asbp_top_down_char (cast `/Game/Character/BP_TopDownChar` OtherActor))
      (if (`KismetSystemLibrary.IsValid` _asbp_top_down_char)
        (`self.K2_DestroyActor`)
        (bind _asbp_hud (cast `/Game/Blueprint/BP_HUD` (`PlayerController.GetHUD` (`GameplayStatics.GetPlayerController` 0))))
        (`/Game/Blueprint/WBP_ScoreWidget.IncrementScore` (`/Game/Blueprint/BP_HUD.ScoreWidgetReference` _asbp_hud))))))

(fn `UserConstructionScript`
  ;[1 1 1] Scale Collision to sprite size
  (`BoxComponent.SetBoxExtent` (`self.PickupCollision`) (* (`.BoxExtent` (`KismetSystemLibrary.GetComponentBounds` (`self.PickupSprite`))) 1.2) true))