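; Actor component that builds or breaks straight, tile-snapped walls outward from its owner in four directions.
; BuildOrBreakWall checks the adjacent tile, then breaks the line if a BP_Building is there, otherwise builds one from the given class.
; Both loops advance tile by tile via a direction-to-vector map set on BeginPlay, stopping at the first failure.
; Tile occupancy comes from a WorldDynamic box overlap that ignores the owner.
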(event `self.ReceiveBeginPlay`
  (set `self.Direction to shift` (`|MakeMap` "NewEnumerator0" (0.0 -1.0) "NewEnumerator1" (0.0 1.0) "NewEnumerator3" (1.0 0.0) "NewEnumerator2" (-1.0 0.0) :!type "/Game/Character/E_PlayerDirection Enum" :!valuetype "Vector2D Structure")))

(fn `Break Wall at Direction`
  (params (LengthInTiles :type Integer :default 10) (Direction :type "/Game/Character/E_PlayerDirection Enum" :default "NewEnumerator3") (`Tile Size` :type Integer :default 32))
  (returns (Complete :type Boolean))
  (locals (Offset :type "Vector Structure" :default (0.0 0.0 0.0)))
  (for _index (range 1 (+ (`local.LengthInTiles`) 1))
    (bind _breakcomplete (`self.BreakAtLocation` (+ (* (`BlueprintMapLibrary.Map_Find` (`self.Direction To Shift`) (`local.Direction`)) _index (`local.Tile Size`)) (+ (`Actor.K2_GetActorLocation` (`self.GetOwner`)) (`self.OffsetForTileMap`)) (`local.Offset`)) (`local.Tile Size`)))
    (if (not _breakcomplete)
      (break)))
  (if true
    (return true)
    (else
      (return false))))

(fn `BreakAtLocation`
  (params (OriginalLocation :type "Vector Structure") (TileSize :type Integer :default 32))
  (returns (BreakComplete :type Boolean))
  (bind (_isbuildingblock _buildinblock) (`self.IsBuildingBlockAtLocation` OriginalLocation TileSize))
  (if _isbuildingblock
    (`Actor.K2_DestroyActor` _buildinblock)
    (return true)
    (else
      (return false))))

(fn `BuildAtLocation`
  (params (OriginalLocation :type "Vector Structure") (TileSize :type Integer :default 32) (ObjectToBuild :type "Actor Class Reference"))
  (returns (isBuildPossible :type Boolean))
  (bind _snapped_location (`/Game/Blueprint/BP_Utilities.SnapToGrid` OriginalLocation TileSize))
  (bind _isfreetile (`self.IsFreeTile` OriginalLocation (`local.TileSize`)))
  (if _isfreetile
    (`|SpawnActorFromClass` (`local.ObjectToBuild`) (`KismetMathLibrary.MakeTransform` _snapped_location) "AlwaysSpawn" "MultiplyWithRoot" null null)
    (return true)
    (else
      (return false))))

(fn `BuildOrBreakWall`
  (params (Direction :type "/Game/Character/E_PlayerDirection Enum" :default "NewEnumerator3") (`Tile Size` :type Integer :default 32) (LengthInTiles :type Integer :default 10) (ObjectToBuild :type "Actor Class Reference"))
  (bind _isbuildingblock (`self.IsBuildingBlockAtLocation` (+ (* (`BlueprintMapLibrary.Map_Find` (`self.Direction To Shift`) (`local.Direction`)) (`local.Tile Size`)) (+ (`Actor.K2_GetActorLocation` (`self.GetOwner`)) (`self.OffsetForTileMap`))) (`local.Tile Size`)))
  (if _isbuildingblock
    (`self.Break Wall at Direction` (`local.LengthInTiles`) (`local.Direction`) (`local.Tile Size`))
    (else
      (`self.BuildWallAtDirection` (`local.LengthInTiles`) (`local.Direction`) (`local.Tile Size`) (`local.ObjectToBuild`)))))

(fn `BuildWallAtDirection`
  (params (LengthInTiles :type Integer :default 10) (Direction :type "/Game/Character/E_PlayerDirection Enum" :default "NewEnumerator3") (`Tile Size` :type Integer :default 32) (ObjectToBuild :type "Actor Class Reference"))
  (returns (Complete :type Boolean))
  (locals (Offset :type "Vector Structure" :default (0.0 0.0 0.0)))
  (for _index (range 1 (+ (`local.LengthInTiles`) 1))
    (bind _isbuildpossible (`self.BuildAtLocation` (+ (* (`BlueprintMapLibrary.Map_Find` (`self.Direction To Shift`) (`local.Direction`)) _index (`local.Tile Size`)) (`Actor.K2_GetActorLocation` (`self.GetOwner`)) (`local.Offset`)) (`local.Tile Size`) (`local.ObjectToBuild`)))
    (if (not _isbuildpossible)
      (break)))
  (if _isbuildpossible
    (return true)
    (else
      (return false))))

(fn `IsBuildingBlock`
  (params (Object :type "Object Object Reference"))
  (returns (IsBuildingBlock :type Boolean))
  (bind _asbp_building (cast `/Game/Blueprint/BP_Building` Object))
  (return (`KismetSystemLibrary.IsValid` _asbp_building)))

(fn `IsBuildingBlockAtLocation`
  (params (Location :type "Vector Structure") (`Tile Size` :type Integer :default 32))
  (returns (IsBuildingBlock :type Boolean) (BuildinBlock :type "Actor Object Reference"))
  (bind (_isfreetile _overlapactors) (`self.IsFreeTile` Location `Tile Size`))
  (if (not _isfreetile)
    (for _array_element _overlapactors
      (bind _isbuildingblock (`self.IsBuildingBlock` _array_element))
      (if _isbuildingblock
        (break)))
    (if _isbuildingblock
      (return true _array_element)
      (else
        (return false _array_element)))))

(fn `IsFreeTile`
  (params (Location :type "Vector Structure") (`Tile Size` :type Integer :default 32))
  (returns (IsFreeTile :type Boolean) (OverlapActors :type "Array of Actor Object Reference"))
  (locals (Offset :type "Vector Structure" :default (0.0 -10.0 0.0)))
  (bind _returnvalue (/ (`local.Tile Size`) 3))
  (bind _snapped_location (`/Game/Blueprint/BP_Utilities.SnapToGrid` Location `Tile Size`))
  (bind (_outactors _returnvalue_2) (`KismetSystemLibrary.BoxOverlapActors` (+ _snapped_location (`local.Offset`)) (`KismetMathLibrary.MakeVector` _returnvalue _returnvalue _returnvalue) (`|MakeArray` "ObjectTypeQuery2" :!type "EObjectTypeQuery Enum") null (`|MakeArray` (`self.GetOwner`))))
  (if _returnvalue_2
    (return false _outactors)
    (else
      (return true))))