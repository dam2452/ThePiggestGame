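; BP_MovingPickup is a pickup that wanders randomly across a Paper2D tile map.
; BeginPlay reads the first tile map's size and starts a looping ChangeDirection timer, its interval randomized once, that picks random XY directions.
; Tick moves it by direction and speed, clamps it to the map bounds at zero Z, and sweeps to the new location.
; An unfinished sphere-trace bounce, marked TODO, is left unconnected.
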(event `self.ReceiveBeginPlay`
  (`parent.ReceiveBeginPlay`)
  (bind _outactors (`GameplayStatics.GetAllActorsOfClass` "/Script/Paper2D.PaperTileMapActor"))
  (bind _tilemap (`PaperTileMapComponent.TileMap` (`PaperTileMapActor.RenderComponent` (`|GetArrayItem` _outactors))))
  (bind _output_get (set `self.Last Map Row` (`PaperTileMap.MapHeight` _tilemap)))
  (`/Engine/EditorBlueprintResources/StandardMacros.DecrementInt` _output_get
    (:`  `
      (bind _output_get_2 (set `self.Last Map Column` (`PaperTileMap.MapWidth` _tilemap)))
      (`/Engine/EditorBlueprintResources/StandardMacros.DecrementInt` _output_get_2
        (:`  `
          (`KismetSystemLibrary.K2_SetTimer` null "ChangeDirection" (`KismetMathLibrary.RandomFloatInRange` (`self.MinTimeToChangeDirection`) (`self.MaxTimeToChangeDirection`)) true))))))

(event `self.ReceiveTick`
  (params (DeltaSeconds :type "Float (single-precision)"))
  (bind (_newlocation_x _newlocation_y) (`KismetMathLibrary.BreakVector` (`self.NewLocation`)))
  (`parent.ReceiveTick` DeltaSeconds)
  (set `self.NewLocation` (+ (* (`self.CurrentDirection`) (`self.MovementSpeed`) DeltaSeconds) (`self.K2_GetActorLocation`)))
  (bind _tile_size (`/Game/Blueprint/BP_Utilities.Get Tile Size`))
  (bind _output_get (set `self.NewLocation` (`KismetMathLibrary.MakeVector` (`KismetMathLibrary.FClamp` _newlocation_x 0.0 (`KismetMathLibrary.Conv_IntToDouble` (* (break `IntPoint` _tile_size) (`self.Last Map Column`)))) (`KismetMathLibrary.FClamp` _newlocation_y 0.0 (`KismetMathLibrary.Conv_IntToDouble` (* (`.Y` (break `IntPoint` _tile_size)) (`self.Last Map Row`)))))))
  (`self.K2_SetActorLocation` _output_get true))

(fn `ChangeDirection`
  (bind (_returnvalue_x _returnvalue_y) (`KismetMathLibrary.BreakVector` (`KismetMathLibrary.RandomUnitVector`)))
  (bind (_returnvalue_x_2 _returnvalue_y_2) (`KismetMathLibrary.BreakVector` (`KismetMathLibrary.Normal` (`KismetMathLibrary.MakeVector` _returnvalue_x _returnvalue_y))))
  (set `self.CurrentDirection` (`KismetMathLibrary.MakeVector` _returnvalue_x_2 _returnvalue_y_2)))

(fn `UserConstructionScript`
  (`parent.UserConstructionScript`))